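; BP_Plot_01 is a satellite actor that moves along an ellipse in the XY plane and plots its trail.
; BeginPlay derives orbital values from element inputs, including angles in radians and a cube-root semi-major-axis calculation, but the movement ignores them.
; Each Tick, SatteliteMovement sets a world location around the origin using sine and cosine of game time, scaled by Speed, Width and Height.
; Temporary red debug points mark the path.
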(event `self.ReceiveBeginPlay`
  (bind _returnvalue (* (`KismetMathLibrary.GetPI`) 2.0))
  (set `self.LongitudeOfTheAscendingNode` (* (`self.RAAN`) (/ (`KismetMathLibrary.GetPI`) 180.0)))
  (set `self.ArgumentOfPeriapsis` (* (`self.argument of perigee`) (/ (`KismetMathLibrary.GetPI`) 180.0)))
  (set `self.meanmotion_rad` (* (`self.mean motion`) (* (/ 1.0 86.400002) _returnvalue)))
  (bind _output_get (set `self.T` (* (`self.meanmotion_rad`) _returnvalue)))
  (set `self.a` (`KismetMathLibrary.MultiplyMultiply_FloatFloat` (/ (* (`KismetMathLibrary.Square` _output_get) (`self.u`)) (* 4.0 (`KismetMathLibrary.Square` (`KismetMathLibrary.GetPI`)))) (/ 1.0 3.0)))
  (set `self.mean anomaly_rad` (`KismetMathLibrary.DegreesToRadians` (`self.mean anomaly`))))

(event `self.ReceiveTick`
  (params (DeltaSeconds :type "Float (single-precision)"))
  (`self.SatteliteMovement`))

(fn `SatteliteMovement`
  (bind _returnvalue (* (`KismetSystemLibrary.GetGameTimeInSeconds`) (`self.Speed`)))
  (bind _returnvalue_2 (`KismetMathLibrary.MakeVector` (* (`KismetMathLibrary.DegSin` _returnvalue) (`self.Width`)) (* (`KismetMathLibrary.DegCos` _returnvalue) (`self.Height`))))
  (`self.K2_SetActorLocation` _returnvalue_2)
  (`KismetSystemLibrary.DrawDebugPoint` _returnvalue_2 5.0 (struct :`R` 1.0 :`B` 0.149277 :`A` 1.0) 10.0))

(fn `UserConstructionScript`)