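; Satellite orbit plotting actor that moves Sphere1 around a circle and leaves short-lived red debug points.
; A Tick event runs OrbitPlot, using sine and cosine of game time times Speed at radius EarthDiameter plus Altitude.
; The construction script sets spring arm length and rotation.
; SatteliteMovement derives an elliptical orbit from UTC time and orbital elements but is not called here; the element conversion and timer setup are disconnected.
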(event `self.ReceiveBeginPlay`)

(event `Tick`)

(event `self.ReceiveTick`
  (params (DeltaSeconds :type "Float (single-precision)"))
  (`self.OrbitPlot`))

(fn `OrbitPlot`
  (bind _sphere1 (`self.Sphere1`))
  (bind _returnvalue (* (`KismetSystemLibrary.GetGameTimeInSeconds`) (`self.Speed`)))
  (bind _returnvalue_2 (+ (`self.EarthDiameter`) (`self.Altitude`)))
  (`SceneComponent.K2_SetRelativeLocation` _sphere1 (`KismetMathLibrary.MakeVector` 0.0 (* (`KismetMathLibrary.DegSin` _returnvalue) _returnvalue_2) (* (`KismetMathLibrary.DegCos` _returnvalue) _returnvalue_2)) false false)
  (`KismetSystemLibrary.DrawDebugPoint` (`SceneComponent.K2_GetComponentLocation` _sphere1) 5.0 (struct :`R` 1.0 :`A` 1.0) 5.0))

(fn `SatteliteMovement`
  (returns (ReturnValue :type "Vector Structure"))
  (bind (_returnvalue_year _returnvalue_month _returnvalue_day _returnvalue_hour _returnvalue_minute _returnvalue_second _returnvalue_millisecond) (`KismetMathLibrary.BreakDateTime` (`KismetMathLibrary.UtcNow`)))
  (bind _eccentricity (`self.eccentricity`))
  (bind _returnvalue (* (`KismetMathLibrary.GetTotalDays` (`KismetMathLibrary.MakeTimespan` (+ _returnvalue_day 213) _returnvalue_hour _returnvalue_minute _returnvalue_second _returnvalue_millisecond)) (`self.Speed`) 360.0))
  (`KismetSystemLibrary.PrintString` (`KismetStringLibrary.Concat_StrStr` (`KismetStringLibrary.Conv_DoubleToString` _returnvalue) "Day: " (`KismetStringLibrary.Conv_IntToString` _returnvalue_day) " - Hour: " (`KismetStringLibrary.Conv_IntToString` _returnvalue_hour) " - Minutes: " (`KismetStringLibrary.Conv_IntToString` _returnvalue_minute) " - Seconds: " (`KismetStringLibrary.Conv_IntToString` _returnvalue_second)))
  (set `SpringArmComponent.TargetArmLength` (/ (* (`self.a`) (- 1.0 _eccentricity)) (+ 1.0 (* _eccentricity (`KismetMathLibrary.DegCos` _returnvalue)))) (`self.SpringArm`))
  (`SceneComponent.K2_SetRelativeRotation` (`self.SpringArm`) (`KismetMathLibrary.MakeRotator` 0.0 0.0 _returnvalue) false false)
  (`self.K2_SetActorRotation` (`KismetMathLibrary.MakeRotator` (`self.inclination`) (`self.argument of perigee`)))
  (return (`SceneComponent.K2_GetComponentLocation` (`self.Sphere`))))

(fn `UserConstructionScript`
  (set `SpringArmComponent.TargetArmLength` (+ (`self.EarthDiameter`) (`self.Altitude`)) (`self.SpringArm`))
  (`SceneComponent.K2_SetRelativeRotation` (`self.SpringArm1`) (`self.ArmRotation`) false false))