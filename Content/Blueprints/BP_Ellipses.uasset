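; Orbital mechanics Blueprint that computes position and velocity on an elliptical orbit when the 9 key is pressed.
; It derives a mean motion from the gravitational parameter and semi-major axis, then solves Kepler's equation for eccentric anomaly by Newton-Raphson iteration.
; That anomaly gives in-plane P/Q coordinates and their rates in meters and seconds, stored in variables alongside the anomaly in degrees.
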(event `Key|Nine`
  (params (Key :type "Key Structure"))
  (:`Pressed`
    (bind _output_get (set `self.mu` (* (`self.mu_min`) (`KismetMathLibrary.MultiplyMultiply_FloatFloat` 10.0 14.0))))
    (bind _output_get_2 (set `self.n_rad_per_s` (* (/ (`self.mu`) (`self.a_km`)) 1000.0)))
    (set `self.n_deg_per_s` (`KismetMathLibrary.RadiansToDegrees` _output_get_2))
    (bind _output_get_3 (set `self.M_Rad` (`KismetMathLibrary.DegreesToRadians` (`self.M_deg`))))
    (set `self.E_Rad` _output_get_3)
    (while (> (`KismetMathLibrary.Abs` (`self.dE`)) (`self.eps`))
      (bind _output_get_4 (set `self.dE` (/ (- (- (`self.E_Rad`) (* (`self.e`) (`KismetMathLibrary.Sin` (`self.E_Rad`)))) (`self.M_Rad`)) (- 1.0 (* (`self.e`) (`KismetMathLibrary.Cos` (`self.E_Rad`)))))))
      (set `self.E_Rad` (- (`self.E_Rad`) _output_get_4)))
    (set `self.p_m` (* (`self.a_km`) 1000.0 (- (`KismetMathLibrary.Cos` (`self.E_Rad`)) (`self.e`))))
    (set `self.q_m` (* (* (`self.a_km`) 1000.0) (`KismetMathLibrary.Sqrt` (- 1.0 (`KismetMathLibrary.MultiplyMultiply_FloatFloat` (`self.e`) 2.0))) (`KismetMathLibrary.Sin` (`self.E_Rad`))))
    (bind _output_get_5 (set `self.dMdt_rad_per_s` (`self.n_rad_per_s`)))
    (bind _output_get_6 (set `self.dEdt_rad_per_s` (/ _output_get_5 (- 1.0 (* (`self.e`) (`KismetMathLibrary.Cos` (`self.E_Rad`)))))))
    (set `self.dpdt_m_per_s` (* _output_get_6 (* (`self.a_km`) -1000.0 (`KismetMathLibrary.Sin` (`self.E_Rad`)))))
    (set `self.dqdt_m_per_s` (* (* (`self.a_km`) 1000.0 (`KismetMathLibrary.Cos` (`self.E_Rad`))) (* (`self.dEdt_rad_per_s`) (`KismetMathLibrary.Sqrt` (- 1.0 (`KismetMathLibrary.MultiplyMultiply_FloatFloat` (`self.e`) 2.0))))))
    (set `self.E_deg_epoch` (`KismetMathLibrary.RadiansToDegrees` (`self.E_Rad`)))))

(fn `UserConstructionScript`)