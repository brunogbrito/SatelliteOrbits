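; Satellite actor that plots one satellite's orbit from a data table of orbital elements, looked up by NORID.
; BeginPlay caches the elements, parsing mean motion and epoch from TLE lines, and enables Tick if the global time reference is valid.
; SatelliteMovement turns day-of-year time into a linear orbit angle, setting spring arm length by the ellipse equation and yaw.
; Actor rotation applies inclination and ascending node; epoch is unused in movement.
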(event `self.ReceiveBeginPlay`
  (bind _returnvalue (`|GetDataTableRow` "/Game/Data/GP_Data_28_8_2021.GP_Data_28_8_2021" (`self.NOR_ID`))
    (:`then`
      (bind _output_get (set `self.Sat_Data` _returnvalue))
      (set `self.OBJECT NAME` (`.OBJECT_NAME_47_C06BD2AE455DE4C3951133BE82C0380F` (break `/Game/Data/GP_Struct_01` _output_get)))
      (set `self.Period` (`KismetStringLibrary.Conv_StringToDouble` (`|GetArrayItem` (`KismetStringLibrary.ParseIntoArray` (`.TLE_LINE2_43_3F8824B04D2C78195613CD9C83416B5D` (break `/Game/Data/GP_Struct_01` _output_get))) 7)))
      (set `self.eccentricity` (`.ECCENTRICITY_20_2260FB2D43E38657D29611BD3861C584` (break `/Game/Data/GP_Struct_01` _output_get)))
      (set `self.inclination` (`.INCLINATION_11_11B299014149FDEB2FFD4C9745A48559` (break `/Game/Data/GP_Struct_01` _output_get)))
      (set `self.argument of perigee` (`.ARG_OF_PERICENTER_24_9A6F696E4B2650EBE334A9A4E3187F60` (break `/Game/Data/GP_Struct_01` _output_get)))
      (set `self.Epoch` (`KismetStringLibrary.Conv_StringToDouble` (`KismetStringLibrary.GetSubstring` (`|GetArrayItem` (`KismetStringLibrary.ParseIntoArray` (`.TLE_LINE1_41_9CA935624CBAD5B6AF8DD09299E116B5` (break `/Game/Data/GP_Struct_01` _output_get))) 3) 2 12)))
      (set `self.SemimajorAxis` (`.SEMIMAJOR_AXIS_30_8B3A842D4C96961A70E832B22143CF40` (break `/Game/Data/GP_Struct_01` _output_get)))
      (set `self.LongitudeOfTheAscendingNode` (`.RA_OF_ASC_NODE_22_EB5537E546EC103CCCB444873AA93744` (break `/Game/Data/GP_Struct_01` _output_get)))
      (`/Engine/EditorBlueprintResources/StandardMacros.IsValid` (`self.GlobalTimeRef`)
        (:`Is Valid`
          (set `self.Condition` true))
        (:`Is Not Valid`
          (`KismetSystemLibrary.PrintString` "Missing Global Time" true true (struct :`R` 1.0 :`B` 0.055224 :`A` 1.0) 10.0))))))

(event `self.ReceiveTick`
  (params (DeltaSeconds :type "Float (single-precision)"))
  (if (`self.Condition`)
    (`self.Satellite Movement` (`/Game/Blueprints/BP_GlobalTime.Date_Output` (`self.GlobalTimeRef`)))))

(fn `Satellite Movement`
  (params (InDateTime :type "DateTime Structure"))
  (returns (SatellitePositon :type "Vector Structure") (SemiMajorAxis :type "Float (double-precision)") (Z_Offset :type "Float (double-precision)") (inclination :type "Float (double-precision)") (LongitudeOfTheAscendingNode :type "Float (double-precision)") (`argument of perigee` :type "Float (double-precision)"))
  (bind (_year _month _day _hour _minute _second _millisecond) (`KismetMathLibrary.BreakDateTime` InDateTime))
  (bind _eccentricity (`self.eccentricity`))
  (bind _longitudeoftheascendingnode (`self.LongitudeOfTheAscendingNode`))
  (bind _inclination (`self.inclination`))
  (bind _returnvalue (* (+ (`KismetMathLibrary.Conv_IntToDouble` (`KismetMathLibrary.GetDayOfYear` InDateTime)) (/ (`KismetMathLibrary.GetTotalMinutes` (`KismetMathLibrary.MakeTimespan` 0 _hour _minute _second _millisecond)) 1440.0)) (`self.Period`) -360.0))
  (bind _returnvalue_2 (+ _returnvalue (`self.Offset_Z_Rotation`) (`self.argument of perigee`)))
  (bind _returnvalue_3 (/ (* (`self.SemimajorAxis`) (- 1.0 _eccentricity)) (+ 1.0 (* _eccentricity (`KismetMathLibrary.DegCos` _returnvalue)))))
  (set `SpringArmComponent.TargetArmLength` _returnvalue_3 (`self.SpringArm`))
  (`SceneComponent.K2_SetRelativeRotation` (`self.SpringArm`) (`KismetMathLibrary.MakeRotator` 0.0 0.0 _returnvalue_2) false false)
  (`self.K2_SetActorRotation` (`KismetMathLibrary.MakeRotator` _inclination (`self.New Rotation Y (Pitch)`) (+ _longitudeoftheascendingnode (`self.New Rotation Z (Yaw)`))))
  (return (`SceneComponent.K2_GetComponentLocation` (`self.Sphere`)) _returnvalue_3 _returnvalue_2 _inclination _longitudeoftheascendingnode (`self.argument of perigee`)))

(fn `UserConstructionScript`)