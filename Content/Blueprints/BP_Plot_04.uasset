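; Satellite actor that plots an orbit from orbital elements and TLE epoch in a data table row keyed by NORID.
; Each tick, two spring arms serve as radius and angle of a simplified ellipse, tilted by inclination and ascending node.
; One follows UTC time since epoch, the other scaled game time.
; Debug points trace both: red on a looping timer for real time, green every tick for game time.
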(event `self.ReceiveBeginPlay`
  (bind _returnvalue (`|GetDataTableRow` "/Game/Data/GP_Data_28_8_2021.GP_Data_28_8_2021" (`self.NOR_ID`))
    (:`then`
      (bind _output_get (set `self.Sat_Data` _returnvalue))
      (set `self.OBJECT NAME` (`.OBJECT_NAME_47_C06BD2AE455DE4C3951133BE82C0380F` (break `/Game/Data/GP_Struct_01` _output_get)))
      (set `self.Period` (/ 1440.0 (`.PERIOD_32_E8EB9E0F48C0C2DEE9DEE2A520392FBF` (break `/Game/Data/GP_Struct_01` _output_get))))
      (set `self.eccentricity` (`.ECCENTRICITY_20_2260FB2D43E38657D29611BD3861C584` (break `/Game/Data/GP_Struct_01` _output_get)))
      (set `self.inclination` (`.INCLINATION_11_11B299014149FDEB2FFD4C9745A48559` (break `/Game/Data/GP_Struct_01` _output_get)))
      (set `self.argument of perigee` (`.ARG_OF_PERICENTER_24_9A6F696E4B2650EBE334A9A4E3187F60` (break `/Game/Data/GP_Struct_01` _output_get)))
      (set `self.Apoapsis` (`.APOAPSIS_34_A801B5E54922829E0A5DB99DEA907AA7` (break `/Game/Data/GP_Struct_01` _output_get)))
      (set `self.Epoch` (`KismetStringLibrary.Conv_StringToDouble` (`KismetStringLibrary.GetSubstring` (`|GetArrayItem` (`KismetStringLibrary.ParseIntoArray` (`.TLE_LINE1_41_9CA935624CBAD5B6AF8DD09299E116B5` (break `/Game/Data/GP_Struct_01` _output_get))) 3) 2 12)))
      (set `self.SemimajorAxis` (`.SEMIMAJOR_AXIS_30_8B3A842D4C96961A70E832B22143CF40` (break `/Game/Data/GP_Struct_01` _output_get)))
      (set `self.LongitudeOfTheAscendingNode` (`.RA_OF_ASC_NODE_22_EB5537E546EC103CCCB444873AA93744` (break `/Game/Data/GP_Struct_01` _output_get)))
      (`KismetSystemLibrary.K2_SetTimerDelegate` (delegate `Tick`) 0.1 true)
      (set `self.Condition` true))))

(event `Tick`
  (`KismetSystemLibrary.DrawDebugPoint` (stale `self.ReceiveTick` _returnvalue) 5.0 (struct :`R` 1.0 :`A` 1.0) 600.0))

(event `self.ReceiveTick`
  (params (DeltaSeconds :type "Float (single-precision)"))
  (if (`self.Condition`)
    (bind _returnvalue (`self.Sattelite Movement`))))

(fn `Sattelite Movement`
  (returns (ReturnValue :type "Vector Structure"))
  (bind (_returnvalue_year _returnvalue_month _returnvalue_day _returnvalue_hour _returnvalue_minute _returnvalue_second _returnvalue_millisecond) (`KismetMathLibrary.BreakDateTime` (`KismetMathLibrary.UtcNow`)))
  (bind _eccentricity (`self.eccentricity`))
  (bind _eccentricity_2 (`self.eccentricity`))
  (bind _returnvalue (* (`KismetSystemLibrary.GetGameTimeInSeconds`) (`self.Period`) 10.0))
  (bind _returnvalue_2 (- (+ (`KismetMathLibrary.Conv_IntToDouble` (`KismetMathLibrary.GetDayOfYear` (`KismetMathLibrary.UtcNow`))) (/ (`KismetMathLibrary.GetTotalSeconds` (`KismetMathLibrary.MakeTimespan` 0 _returnvalue_hour _returnvalue_minute _returnvalue_second _returnvalue_millisecond)) 86400.0)) (`self.Epoch`)))
  (bind _returnvalue_3 (* _returnvalue_2 (`self.Period`) 360.0))
  (`KismetSystemLibrary.PrintString` (`KismetStringLibrary.Concat_StrStr` "Name: " (`self.OBJECT NAME`) "  |  Current Clock:" (`KismetStringLibrary.Conv_DoubleToString` _returnvalue_2)))
  (set `SpringArmComponent.TargetArmLength` (/ (* (`self.SemimajorAxis`) (- 1.0 _eccentricity)) (+ 1.0 (* _eccentricity (`KismetMathLibrary.DegCos` _returnvalue_3)))) (`self.SpringArm`))
  (`SceneComponent.K2_SetRelativeRotation` (`self.SpringArm`) (`KismetMathLibrary.MakeRotator` 0.0 0.0 (+ _returnvalue_3 (`self.Offset`))) false false)
  (set `SpringArmComponent.TargetArmLength` (/ (* (`self.SemimajorAxis`) (- 1.0 _eccentricity_2)) (+ 1.0 (* _eccentricity_2 (`KismetMathLibrary.DegCos` _returnvalue)))) (`self.SpringArm1`))
  (`SceneComponent.K2_SetRelativeRotation` (`self.SpringArm1`) (`KismetMathLibrary.MakeRotator` 0.0 0.0 (+ _returnvalue (`self.Offset`))) false false)
  (`self.K2_SetActorRotation` (`KismetMathLibrary.MakeRotator` (`self.inclination`) 180.0 (`self.LongitudeOfTheAscendingNode`)))
  (`KismetSystemLibrary.DrawDebugPoint` (`SceneComponent.K2_GetComponentLocation` (`self.Sphere1`)) 2.5 (struct :`G` 1.0 :`B` 0.065609 :`A` 1.0) 360.0)
  (return (`SceneComponent.K2_GetComponentLocation` (`self.Sphere`))))

(fn `UserConstructionScript`)