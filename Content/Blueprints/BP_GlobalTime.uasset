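; BP_GlobalTime is a Blueprint that keeps a shared date and time value for the game.
; Each Tick it writes DateOutput from either the current UTC clock or, when DebugMode is on, a fixed date built from debug year-to-second variables.
; The debug override has zero milliseconds, and the construction script is empty.
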(event `self.ReceiveTick`
  (params (DeltaSeconds :type "Float (single-precision)"))
  (bind (_year _month _day _hour _minute _second _millisecond) (`KismetMathLibrary.BreakDateTime` (select `bool` (`self.DebugMode`) :`false` (`KismetMathLibrary.UtcNow`) :`true` (`KismetMathLibrary.MakeDateTime` (`self.Debug_Year`) (`self.Debug_Month`) (`self.Debug_Day`) (`self.Debug_Hour`) (`self.Debug_Minute`) (`self.Debug_Second`)))))
  (set `self.Date_Output` (`KismetMathLibrary.MakeDateTime` _year _month _day _hour _minute _second _millisecond)))

(fn `UserConstructionScript`)