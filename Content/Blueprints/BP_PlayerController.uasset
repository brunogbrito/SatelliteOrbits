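; BP_PlayerController is a player controller that queries the N2YO satellite tracking web API through the VaRest plugin.
; BeginPlay constructs a GET request and binds its completion and failure events.
; Pressing the 0 key sets a satellite id field on the request and sends it to the API URL with the key appended.
; Completion prints the response as a string, while failure displays nothing.
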(event `self.ReceiveBeginPlay`
  (bind _myrequest (`self.MyRequest`))
  (bind _returnvalue (`VaRestSubsystem.ConstructVaRestRequestExt` (subsystem `VaRestSubsystem`) "GET" "x_www_form_urlencoded_url"))
  (set `self.MyRequest` _returnvalue)
  (add `VaRestRequestJSON.OnRequestComplete` _myrequest (delegate `OnRequestComplete_Event_0`))
  (add `VaRestRequestJSON.OnRequestFail` _myrequest (delegate `OnRequestFail_Event_0`)))

(event `OnRequestComplete_Event_0`
  (params (Request :type "VaRestRequestJSON Object Reference"))
  (bind _returnvalue (`VaRestRequestJSON.GetResponseContentAsString` Request true))
  (`KismetSystemLibrary.PrintString` _returnvalue))

(event `OnRequestFail_Event_0`
  (params (Request :type "VaRestRequestJSON Object Reference"))
  (`VaRestRequestJSON.GetResponseContentAsString` Request true))

(event `Key|Zero`
  (params (Key :type "Key Structure"))
  (bind _myrequest (`self.MyRequest`))
  (:`Pressed`
    (`VaRestJsonObject.SetIntegerField` (`VaRestRequestJSON.GetRequestObject` _myrequest) "id" 25544)
    (`VaRestRequestJSON.ProcessURL` _myrequest (`KismetStringLibrary.Concat_StrStr` "https://api.n2yo.com/rest/v1/satellite/v1" (`self.API_Key`)))))

(fn `UserConstructionScript`)