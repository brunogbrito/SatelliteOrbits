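; BP_Earth is an Earth actor that spins in yaw to match the simulated date and time.
; On BeginPlay it finds the BP_GlobalTime actor, printing an error if none exists.
; Each Tick turns that clock's date into fractional days of the year and scales them by a sidereal-style rate of just over one negative turn per day.
; An offset and an extra day-of-year correction complete the absolute yaw.
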(event `self.ReceiveBeginPlay`
  (bind _outactors (`GameplayStatics.GetAllActorsOfClass` "/Game/Blueprints/BP_GlobalTime.BP_GlobalTime_C"))
  (bind _output (`|GetArrayItem` _outactors))
  (`/Engine/EditorBlueprintResources/StandardMacros.IsValid` _output
    (:`Is Valid`
      (set `self.GlobalTimeRef` _output))
    (:`Is Not Valid`
      (`KismetSystemLibrary.PrintString` "Missing Global Time" true true (struct :`R` 1.0 :`B` 0.055224 :`A` 1.0) 10.0))))

(event `self.ReceiveTick`
  (params (DeltaSeconds :type "Float (single-precision)"))
  (bind _globaltimeref (`self.GlobalTimeRef`)
    (:`then`
      (bind _date_output (`/Game/Blueprints/BP_GlobalTime.Date_Output` _globaltimeref))
      (bind _returnvalue (`KismetMathLibrary.GetDayOfYear` _date_output))
      (bind (_year _month _day _hour _minute _second _millisecond) (`KismetMathLibrary.BreakDateTime` _date_output))
      (bind _returnvalue_2 (/ (`KismetMathLibrary.GetTotalMinutes` (`KismetMathLibrary.MakeTimespan` _returnvalue _hour _minute _second _millisecond)) 1440.0))
      (`self.K2_SetActorRotation` (`KismetMathLibrary.MakeRotator` 0.0 0.0 (+ (* _returnvalue_2 -360.984985) (`self.Earth_Rotation_Offset`) (* _returnvalue -4.0))))
      (`KismetSystemLibrary.PrintString` (`KismetStringLibrary.Conv_DoubleToString` _returnvalue_2) false false))
    (:`else`)))

(fn `UserConstructionScript`)