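; Test Blueprint for satellite TLE data access that prints debug results to screen.
; BeginPlay constructs a VaRest GET request and binds response-printing callbacks, but the nodes that would send it are unconnected.
; Pressing 0 reads the Zarya row from a GP data table, extracts the TLE epoch and prints it with its offset in days from current UTC.
; Other unconnected fragments sketch API calls and JSON file loading.
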(event `self.ReceiveBeginPlay`
  (bind _myrequest (`self.MyRequest`))
  (bind _returnvalue (`VaRestSubsystem.ConstructVaRestRequestExt` (subsystem `VaRestSubsystem`) "GET" "json"))
  (set `self.MyRequest` _returnvalue)
  (add `VaRestRequestJSON.OnRequestComplete` _myrequest (delegate `OnRequestComplete_Event_0`))
  (add `VaRestRequestJSON.OnRequestFail` _myrequest (delegate `OnRequestFail_Event_0`)))

(event `OnRequestComplete_Event_0`
  (params (Request :type "VaRestRequestJSON Object Reference"))
  (bind _returnvalue (`VaRestRequestJSON.GetResponseContentAsString` Request true))
  (`KismetSystemLibrary.PrintString` _returnvalue))

(event `OnRequestFail_Event_0`
  (params (Request :type "VaRestRequestJSON Object Reference"))
  (bind _returnvalue (`VaRestRequestJSON.GetResponseContentAsString` Request true))
  (`KismetSystemLibrary.PrintString` _returnvalue))

(event `Key|Zero`
  (params (Key :type "Key Structure"))
  (bind (_returnvalue_year _returnvalue_month _returnvalue_day _returnvalue_hour _returnvalue_minute _returnvalue_second _returnvalue_millisecond) (`KismetMathLibrary.BreakDateTime` (`KismetMathLibrary.UtcNow`)))
  (:`Pressed`
    (bind _returnvalue (`|GetDataTableRow` "/Game/Data/GP_Data_28_8_2021.GP_Data_28_8_2021" (`self.Zarya`))
      (:`then`
        (bind _output (`|GetArrayItem` (`KismetStringLibrary.ParseIntoArray` (`.TLE_LINE1_41_9CA935624CBAD5B6AF8DD09299E116B5` (break `/Game/Data/GP_Struct_01` _returnvalue))) 3))
        (`KismetSystemLibrary.PrintString` (`KismetStringLibrary.Concat_StrStr` _output "   --- Current Clock: " (`KismetStringLibrary.Conv_DoubleToString` (- (+ (`KismetMathLibrary.Conv_IntToDouble` (`KismetMathLibrary.GetDayOfYear` (`KismetMathLibrary.UtcNow`))) (/ (`KismetMathLibrary.GetTotalSeconds` (`KismetMathLibrary.MakeTimespan` 0 _returnvalue_hour _returnvalue_minute _returnvalue_second _returnvalue_millisecond)) 86400.0)) (`KismetStringLibrary.Conv_StringToDouble` (`KismetStringLibrary.GetSubstring` _output 2 12))))) true true (struct :`G` 1.0 :`B` 0.346875 :`A` 1.0) 5.0)))))

(fn `UserConstructionScript`)