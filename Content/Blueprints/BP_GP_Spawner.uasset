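; BP_GP_Spawner populates the level with plot actors for orbital objects listed in the GP_Data_28_8_2021 data table.
; On BeginPlay it caches the BP_GlobalTime actor and walks every table row, skipping object types switched off by the TBA, debris, payload and rocket body exclude flags.
; Each remaining row spawns a BP_Plot_06 at the spawner's own transform, passing the row name as NORID along with the shared time reference.
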(event `self.ReceiveBeginPlay`
  (bind _outactors (`GameplayStatics.GetAllActorsOfClass` "/Game/Blueprints/BP_GlobalTime.BP_GlobalTime_C"))
  (set `self.GlobalTime` (`|GetArrayItem` _outactors))
  (bind _outrownames (`DataTableFunctionLibrary.GetDataTableRowNames` "/Game/Data/GP_Data_28_8_2021.GP_Data_28_8_2021"))
  (for _array_element _outrownames
    (bind _returnvalue (`|GetDataTableRow` "/Game/Data/GP_Data_28_8_2021.GP_Data_28_8_2021" _array_element)
      (:`then`
        (if (not (or (and (`self.Exclude TBA`) (`KismetStringLibrary.EqualEqual_StrStr` (`.OBJECT_TYPE_50_6B15C35C4D4F2E9D838C61891D6E16E6` (break `/Game/Data/GP_Struct_01` _returnvalue)) "TBA")) (and (`self.Exclude Debris`) (`KismetStringLibrary.EqualEqual_StrStr` (`.OBJECT_TYPE_50_6B15C35C4D4F2E9D838C61891D6E16E6` (break `/Game/Data/GP_Struct_01` _returnvalue)) "DEBRIS")) (and (`self.Exclude Playload`) (`KismetStringLibrary.EqualEqual_StrStr` (`.OBJECT_TYPE_50_6B15C35C4D4F2E9D838C61891D6E16E6` (break `/Game/Data/GP_Struct_01` _returnvalue)) "PAYLOAD")) (and (`self.Exclude Rocket Body`) (`KismetStringLibrary.EqualEqual_StrStr` (`.OBJECT_TYPE_50_6B15C35C4D4F2E9D838C61891D6E16E6` (break `/Game/Data/GP_Struct_01` _returnvalue)) "ROCKET BODY"))))
          (`|SpawnActorFromClass` "/Game/Blueprints/BP_Plot_06.BP_Plot_06_C" (`self.GetTransform`) "AlwaysSpawn" "OverrideRootScale" null _array_element (`self.GlobalTime`) null))))))

(fn `UserConstructionScript`)