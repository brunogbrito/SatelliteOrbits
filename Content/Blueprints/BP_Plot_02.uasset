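; Actor that animates a satellite along an elliptical-style orbit and plots its trail with debug points.
; Each tick, a spring arm's yaw follows game time times Speed, its length follows an eccentricity-based radius, and actor rotation applies inclination and argument of perigee.
; A looping timer draws the sphere's returned position.
; Orbital-element conversions, including semi-major axis, never run; UTC time is only printed, alongside the angle.
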(event `self.ReceiveBeginPlay`
  (`KismetSystemLibrary.K2_SetTimerDelegate` (delegate `Tick`) 0.1 true))

(event `Tick`
  (`KismetSystemLibrary.DrawDebugPoint` (stale `self.ReceiveTick` _returnvalue) 5.0 (struct :`R` 1.0 :`A` 1.0) 600.0))

(event `self.ReceiveTick`
  (params (DeltaSeconds :type "Float (single-precision)"))
  (bind _returnvalue (`self.SatteliteMovement`)))

(fn `SatteliteMovement`
  (returns (ReturnValue :type "Vector Structure"))
  (bind (_returnvalue_year _returnvalue_month _returnvalue_day _returnvalue_hour _returnvalue_minute _returnvalue_second _returnvalue_millisecond) (`KismetMathLibrary.BreakDateTime` (`KismetMathLibrary.UtcNow`)))
  (bind _eccentricity (`self.eccentricity`))
  (bind _returnvalue (* (`KismetSystemLibrary.GetGameTimeInSeconds`) (`self.Speed`) 360.0))
  (`KismetSystemLibrary.PrintString` (`KismetStringLibrary.Concat_StrStr` (`KismetStringLibrary.Conv_DoubleToString` _returnvalue) "Day: " (`KismetStringLibrary.Conv_IntToString` _returnvalue_day) " - Hour: " (`KismetStringLibrary.Conv_IntToString` _returnvalue_hour) " - Minutes: " (`KismetStringLibrary.Conv_IntToString` _returnvalue_minute) " - Seconds: " (`KismetStringLibrary.Conv_IntToString` _returnvalue_second)))
  (set `SpringArmComponent.TargetArmLength` (/ (* (`self.a`) (- 1.0 _eccentricity)) (+ 1.0 (* _eccentricity (`KismetMathLibrary.DegCos` _returnvalue)))) (`self.SpringArm`))
  (`SceneComponent.K2_SetRelativeRotation` (`self.SpringArm`) (`KismetMathLibrary.MakeRotator` 0.0 0.0 _returnvalue) false false)
  (`self.K2_SetActorRotation` (`KismetMathLibrary.MakeRotator` (`self.inclination`) (`self.argument of perigee`)))
  (return (`SceneComponent.K2_GetComponentLocation` (`self.Sphere`))))

(fn `UserConstructionScript`)